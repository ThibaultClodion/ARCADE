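; BP_Ball is a ball actor that drives its Sphere component with a simulated slope weight force along the X axis.
; Every Tick applies the result of GetGravityVector to the Sphere through AddForce, as a force rather than an acceleration.
; GetGravityVector multiplies the sphere's mass, Gravity, the sine of AngleInDeg and a WeightForceCorrection factor, leaving Y and Z at zero.
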(event EventTick
  (params (DeltaSeconds :type Float%20%28single-precision%29))
  ;[1 0.9467 0.4478] Apply Weight Force
  (Physics|AddForce (Variables|Default|GetSphere) (CallFunction|GetGravityVector) "None" false))

(fn ConstructionScript)

(fn GetGravityVector
  (return (Math|Vector|MakeVector (* (Physics|GetMass (Variables|Default|GetSphere)) (Variables|Gravity|GetGravity) (Math|Trig|Sin(Degrees) (Variables|Gravity|GetAngleInDeg)) (Variables|Gravity|GetWeightForceCorrection)) 0.0 0.0)))