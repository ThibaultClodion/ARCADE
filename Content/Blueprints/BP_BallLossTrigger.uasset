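; Trigger actor that handles losing a ball, either respawning it or ending the game.
; On BeginPlay it caches the BP_Ball's starting location as the respawn point.
; On any actor overlap it plays a sound, then, if balls remain, moves that actor back to the start, decrements BallLeft and prints the count.
; At zero balls left it quits the game.
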(event EventBeginPlay
  (bind _returnvalue (Actor|GetActorOfClass "/Game/Blueprints/BP_Ball.BP_Ball_C"))
  (Variables|Default|SetBallInitLocation (Transformation|GetActorLocation _returnvalue)))

(event Collision|EventActorBeginOverlap
  (params (OtherActor :type Actor%20Object%20Reference))
  (bind _ballleft (Variables|Default|GetBallLeft))
  (Audio|PlaySound2D "/Game/Effects/arcade-ui-5-229504.arcade-ui-5-229504" 0.25 1.0 0.0 0 0)
  (Math|Integer|CompareInt (Variables|Default|GetBallLeft)
    (:>
      (Transformation|SetActorLocation OtherActor (Variables|Default|GetBallInitLocation) false false)
      (Math|Integer|DecrementInt _ballleft
        (:%20%20
          (Development|PrintString (Utilities|String|Append (Utilities|String|ToString(Integer) _ballleft) " balls left.")))))
    (:==
      (Game|QuitGame 0 "Quit" false))))

(fn ConstructionScript)