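; Player controller that drives the flippers for two players sharing one keyboard.
; On BeginPlay it finds every BP_Flipper in the level and stores each by its FlipperType as a left or right flipper for player one or two.
; Hardcoded key events call Flip on press and Flop on release for the matching flipper, through helper functions that skip invalid references.
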(event EventBeginPlay
  ;[1 1 1] Get flippers
  (bind _outactors (Actor|GetAllActorsOfClass "/Game/Blueprints/BP_Flipper.BP_Flipper_C"))
  (for _array_element _outactors
    (switch Utilities|FlowControl|Switch|SwitchonFlipperType (Variables|/Game/Blueprints/BP_Flipper.BP_Flipper_C|GetFlipperType _array_element)
      (:NewEnumerator0
        (Variables|Default|SetPlayerOne_LeftFlipper _array_element))
      (:NewEnumerator1
        (Variables|Default|SetPlayerOne_RightFlipper _array_element))
      (:NewEnumerator2
        (Variables|Default|SetPlayerTwo_LeftFlipper _array_element))
      (:NewEnumerator3
        (Variables|Default|SetPlayerTwo_RightFlipper _array_element)))))

(event Input|KeyboardEvents|W
  (params (Key :type Key%20Structure :default "None"))
  (bind _playerone_leftflipper (Variables|Default|GetPlayerOne_LeftFlipper))
  ;[1 0.7298 0.3146] FlipFlop - Player One - Left Flipper
  (:Pressed
    (CallFunction|Flip _playerone_leftflipper))
  (:Released
    (CallFunction|Flop _playerone_leftflipper)))

(event Input|KeyboardEvents|C
  (params (Key :type Key%20Structure :default "None"))
  (bind _playerone_rightflipper (Variables|Default|GetPlayerOne_RightFlipper))
  ;[1 0.7298 0.3146] FlipFlop - Player One - Right Flipper
  (:Pressed
    (CallFunction|Flip _playerone_rightflipper))
  (:Released
    (CallFunction|Flop _playerone_rightflipper)))

(event Input|KeyboardEvents|Left
  (params (Key :type Key%20Structure :default "None"))
  (bind _playertwo_leftflipper (Variables|Default|GetPlayerTwo_LeftFlipper))
  ;[0.6402 0.8674 1] FlipFlop - Player Two - Left Flipper
  (:Pressed
    (CallFunction|Flip _playertwo_leftflipper))
  (:Released
    (CallFunction|Flop _playertwo_leftflipper)))

(event Input|KeyboardEvents|Right
  (params (Key :type Key%20Structure :default "None"))
  (bind _playertwo_rightflipper (Variables|Default|GetPlayerTwo_RightFlipper))
  ;[0.6402 0.8674 1] FlipFlop - Player One - Right Flipper
  (:Pressed
    (CallFunction|Flip _playertwo_rightflipper))
  (:Released
    (CallFunction|Flop _playertwo_rightflipper)))

(fn ConstructionScript)

(fn Flop
  (params (Flipper :type BP%20Flipper%20Object%20Reference))
  (if (Utilities|IsValid Flipper)
    (Default|Flop Flipper)))

(fn Flip
  (params (Flipper :type BP%20Flipper%20Object%20Reference))
  (if (Utilities|IsValid Flipper)
    (Default|Flip Flipper)))