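; BP_Elevator1 is a Map4 elevator that acts as a teleporter for the ball.
; Any actor overlapping its Box is destroyed; after a one-second delay a fresh BP_Ball spawns at TeleportLocation and receives a backward force on its Sphere.
; It then prints a "Hello" message and, if Center is false, deactivates its own root and the RoofSide and RoofTop root components.
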(event OnComponentBeginOverlap(Box)
  (params (OverlappedComponent :type Primitive%20Component%20Object%20Reference) (OtherActor :type Actor%20Object%20Reference) (OtherComp :type Primitive%20Component%20Object%20Reference) (OtherBodyIndex :type Integer) (bFromSweep :type Boolean) (SweepResult :type Hit%20Result%20Structure%20%28by%20ref%29))
  (Actor|DestroyActor OtherActor)
  (Utilities|FlowControl|Delay 1.0)
  (bind _returnvalue (Game|SpawnActorfromClass "/Game/Blueprints/BP_Ball.BP_Ball_C" (Math|Transform|MakeTransform (Transformation|GetActorLocation (Variables|Default|GetTeleportLocation)) "0, 0, 0" "1.000000,1.000000,1.000000") "Undefined" "MultiplyWithRoot" 0 0))
  (Physics|AddForce (Variables|/Game/Blueprints/BP_Ball.BP_Ball_C|GetSphere _returnvalue) (Class|KismetMathLibrary|VectorBackward) "None" false)
  (Development|PrintText "Hello")
  (if (not (Variables|Default|GetCenter))
    (Components|Activation|Deactivate (Variables|Default|GetDefaultSceneRoot))))

(fn ConstructionScript)