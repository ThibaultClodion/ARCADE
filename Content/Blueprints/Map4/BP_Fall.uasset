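; BP_Fall is a pinball fall trigger that destroys a BP_Ball on overlapping its box.
; After a one-second delay, it re-activates and shows the roof pieces.
; Unless flagged Center, it also reveals the barriers, ground and tagged actors and teleports four flippers to marker positions.
; That branch then spawns a replacement ball at a teleport point with the saved velocity and moves the camera to a base location.
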(event OnComponentBeginOverlap(Box)
  (params (OverlappedComponent :type Primitive%20Component%20Object%20Reference) (OtherActor :type Actor%20Object%20Reference) (OtherComp :type Primitive%20Component%20Object%20Reference) (OtherBodyIndex :type Integer) (bFromSweep :type Boolean) (SweepResult :type Hit%20Result%20Structure%20%28by%20ref%29))
  (bind _asbp_ball (Utilities|Casting|CastToBP_Ball OtherActor))
  (Variables|Default|SetVitesse (Transformation|GetVelocity _asbp_ball))
  (Actor|DestroyActor OtherActor)
  (Utilities|FlowControl|Delay 1.0)
  (Components|Activation|Activate (Variables|/Script/Engine.Actor|GetRootComponent (Variables|Default|GetRoofTop)) false)
  (if (Variables|Default|GetCenter)
    (Rendering|SetVisibility (Variables|/Script/Engine.Actor|GetRootComponent (Variables|Default|GetRoofTop)) true false)
    (else
      (Rendering|SetVisibility (Variables|/Script/Engine.Actor|GetRootComponent (Variables|Default|GetRoofTop)) true false)
      (bind _outactors (Actor|GetAllActorswithTag "ToDisableActor"))
      (for _array_element _outactors
        (Rendering|SetActorHiddenInGame _array_element false))
      (Transformation|SetActorLocation (Variables|Default|GetFlipperRight1) (Transformation|GetActorLocation (Variables|Default|GetRight1)) false true)
      (Transformation|SetActorLocation (Variables|Default|GetFlipperRight2) (Transformation|GetActorLocation (Variables|Default|GetRight2)) false true)
      (Transformation|SetActorLocation (Variables|Default|GetFlipperLeft1) (Transformation|GetActorLocation (Variables|Default|GetLeft1)) false true)
      (Transformation|SetActorLocation (Variables|Default|GetFlipperLeft2) (Transformation|GetActorLocation (Variables|Default|GetLeft2)) false true)
      (bind _returnvalue (Game|SpawnActorfromClass "/Game/Blueprints/BP_Ball.BP_Ball_C" (Math|Transform|MakeTransform (Transformation|GetActorLocation (Variables|Default|GetTeleportLocation)) "0, 0, 0" "1.000000,1.000000,1.000000") "Undefined" "MultiplyWithRoot" 0 0))
      (Physics|SetPhysicsLinearVelocity (Variables|/Game/Blueprints/BP_Ball.BP_Ball_C|GetSphere _returnvalue) (Variables|Default|GetVitesse) false "None")
      (Default|MoovingCam (Variables|Default|GetCam) (Variables|Default|GetCamera) (Transformation|GetActorLocation (Variables|Default|GetBaseLocation)) false))))

(fn ConstructionScript)