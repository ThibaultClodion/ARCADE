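; CamChange is a trigger actor that repositions a camera when a BP_Ball enters its box.
; After a one-second delay, it snaps PreviousCam to the location of the NewPosition actor, with no interpolation.
; The Rotate flag picks between two hard-coded camera rotations.
; The MoovingCam event runs the same delayed move without needing an overlap.
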(event OnComponentBeginOverlap(Box)
  (params (OverlappedComponent :type Primitive%20Component%20Object%20Reference) (OtherActor :type Actor%20Object%20Reference) (OtherComp :type Primitive%20Component%20Object%20Reference) (OtherBodyIndex :type Integer) (bFromSweep :type Boolean) (SweepResult :type Hit%20Result%20Structure%20%28by%20ref%29))
  (Utilities|Casting|CastToBP_Ball OtherActor)
  (Utilities|FlowControl|Delay 1.0)
  (Transformation|SetActorLocation (Variables|Default|GetPreviousCam) (Transformation|GetActorLocation (Variables|Default|GetNewPosition)) false false)
  (if (Variables|Default|GetRotate)
    (Transformation|SetActorRotation (Variables|Default|GetPreviousCam) "-60.000000,0.000000,0.000000")
    (else
      (Transformation|SetActorRotation (Variables|Default|GetPreviousCam) "-50.000000,0.000000,0.000000"))))

(event Custom|MoovingCam
  (Utilities|FlowControl|Delay 1.0)
  (Transformation|SetActorLocation (Variables|Default|GetPreviousCam) (Transformation|GetActorLocation (Variables|Default|GetNewPosition)) false false)
  (if (Variables|Default|GetRotate)
    (Transformation|SetActorRotation (Variables|Default|GetPreviousCam) "-60.000000,0.000000,0.000000")
    (else
      (Transformation|SetActorRotation (Variables|Default|GetPreviousCam) "-50.000000,0.000000,0.000000"))))

(fn ConstructionScript)