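; Game mode for a flipper (pinball) game that sets up the HUD and spawns the ball when play begins.
; It creates and refreshes the in-game score widget, then spawns BP_Ball at the first PlayerStart found.
; On Map1 and Map3, chosen by level name, it also adds a purifiers widget and sets a WidgetReady flag.
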(event EventBeginPlay
  (CallFunction|CreateScoreWidget)
  (CallFunction|SpawnBall)
  (bind _returnvalue (Game|GetCurrentLevelName true))
  (if (Utilities|Enum|Equal(Enum) _returnvalue "Map3")
    (CallFunction|CreatePurifiersWidget :!label _label)
    (elif (Utilities|Enum|Equal(Enum) _returnvalue "Map1")
      (goto _label))))

(fn ConstructionScript)

(fn CreateScoreWidget
  (bind _returnvalue (UserInterface|CreateWidget "/Game/UI/WBP_InGame.WBP_InGame_C" (Game|GetPlayerController 0)))
  (bind _output_get (Variables|Default|SetScoreWidget _returnvalue))
  (UserInterface|Viewport|AddtoViewport _output_get 0)
  (Default|UpdateAll _output_get))

(fn SpawnBall
  (bind _returnvalue (Actor|GetActorOfClass "/Script/Engine.PlayerStart"))
  (Game|SpawnActorfromClass "/Game/Blueprints/BP_Ball.BP_Ball_C" (Transformation|GetActorTransform _returnvalue) "Undefined" "MultiplyWithRoot" 0 0))

(fn CreatePurifiersWidget
  (bind _returnvalue (UserInterface|CreateWidget "/Game/UI/WBP_Purifiers.WBP_Purifiers_C" (Game|GetPlayerController 0)))
  (bind _output_get (Variables|Default|SetPurifiersWidget _returnvalue))
  (UserInterface|Viewport|AddtoViewport _output_get 0)
  (Variables|Default|SetWidgetReady true))