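; Game instance for a pinball (flipper) game that holds the player score, remaining balls and purifier progress.
; AddScore accumulates points, and BallLoss decrements the balls, then has GameMode_Flipper spawn another and refresh the lives widget.
; When no balls remain, it prints the score as a placeholder for an unimplemented end screen, resets all data and opens the main menu.
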(fn AddScore
  (params (ScoreToAdd :type Integer))
  ;[0.5153 1 0.9301] Add score
  (Variables|Default|SetPlayer%20Score (+ ScoreToAdd (Variables|Default|GetPlayer%20Score))))

(fn BallLoss
  (bind _result (Math|Integer|DecrementInt (Variables|Default|GetNb_Remaining_Balls))
    (:%20%20
      (if (<= _result 0)
        ;[0.1779 1 0.6939] TODO : Implement EndGame and Scoreboard
        (Development|PrintString (Utilities|String|ToString(Integer) (Variables|Default|GetPlayer%20Score)))
        (CallFunction|ResetData)
        (Game|OpenLevel(byObjectReference) "/Game/Maps/MainMenu.MainMenu")
        (else
          (bind _asgame_mode_flipper (Utilities|Casting|CastToGameMode_Flipper (Game|GetGameMode)))
          (Default|SpawnBall _asgame_mode_flipper)
          ;[0.1779 1 0.6939] Calls UI function to update remaining balls
          (Default|UpdateLives (Variables|/Game/Blueprints/Game/GameMode_Flipper.GameMode_Flipper_C|GetScoreWidget _asgame_mode_flipper)))))))

(fn ResetData
  (Variables|Default|SetPlayer%20Score 0)
  (Variables|Default|SetPurifiers 0)
  (Variables|Default|SetPurifiersMap3 0)
  (Variables|Default|SetNb_Remaining_Balls 3)
  (Variables|Default|SetIndex 2)
  (Variables|Default|SetPurifiersCount 0)
  (Variables|Default|SetPurifiersMap3Count 0))