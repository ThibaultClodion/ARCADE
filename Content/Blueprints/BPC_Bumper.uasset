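; BPC_Bumper is an actor component that makes its owner act as a bumper for BP_Ball actors.
; On BeginPlay it binds to the hit event of the owner's root primitive component.
; When a BP_Ball hits, it applies an impulse to the ball's Sphere along the ball-to-owner direction, scaled by ImpulsePower and AdjustPower, so the sign of those values decides push or pull.
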(event Custom|OnRootHit
  (params (HitComponent :type Primitive%20Component%20Object%20Reference) (OtherActor :type Actor%20Object%20Reference) (OtherComp :type Primitive%20Component%20Object%20Reference) (NormalImpulse :type Vector) (Hit :type Hit%20Result%20Structure%20%28by%20ref%29))
  ;[1 0.4596 0.3798] Add impulse on root hit
  (bind _asbp_ball (Utilities|Casting|CastToBP_Ball OtherActor))
  (Physics|AddImpulse (Variables|/Game/Blueprints/BP_Ball.BP_Ball_C|GetSphere _asbp_ball) (* (Math|Vector|GetUnitDirection(Vector) (Transformation|GetActorLocation _asbp_ball) (Transformation|GetActorLocation (Components|GetOwner))) (Variables|Default|GetImpulsePower) (Variables|Default|GetAdjustPower)) "None" false))

(event EventBeginPlay
  ;[0.5204 1 0.7252] Get the owner onHit event
  (bind _asprimitive_component (Utilities|Casting|CastToPrimitiveComponent (Variables|/Script/Engine.Actor|GetRootComponent (Components|GetOwner))))
  (Collision|BindEventtoOnComponentHit _asprimitive_component (delegate Custom|OnRootHit)))