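; BP_River is a river obstacle that switches collision on and off through two trigger volumes.
; Its two walls and cube start with collision disabled on BeginPlay, and OffBox disables them again when the BP_Ball actor overlaps it.
; OnBox restores query and physics collision on any overlap, without checking the actor, and each switch prints a status message.
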(event OnComponentBeginOverlap(OnBox)
  (params (OverlappedComponent :type Primitive%20Component%20Object%20Reference) (OtherActor :type Actor%20Object%20Reference) (OtherComp :type Primitive%20Component%20Object%20Reference) (OtherBodyIndex :type Integer) (bFromSweep :type Boolean) (SweepResult :type Hit%20Result%20Structure%20%28by%20ref%29))
  (Collision|SetCollisionEnabled (Variables|Default|Get%20OnWall) "QueryAndPhysics")
  (Development|PrintText "Enabed river"))

(event OnComponentBeginOverlap(OffBox)
  (params (OverlappedComponent :type Primitive%20Component%20Object%20Reference) (OtherActor :type Actor%20Object%20Reference) (OtherComp :type Primitive%20Component%20Object%20Reference) (OtherBodyIndex :type Integer) (bFromSweep :type Boolean) (SweepResult :type Hit%20Result%20Structure%20%28by%20ref%29))
  (bind _returnvalue (Actor|GetActorOfClass "/Game/Blueprints/BP_Ball.BP_Ball_C"))
  (if (== OtherActor _returnvalue)
    (Collision|SetCollisionEnabled (Variables|Default|Get%20OnWall) "NoCollision")
    (Development|PrintText "Disabled River")))

(event EventBeginPlay
  (Collision|SetCollisionEnabled (Variables|Default|Get%20OnWall) "NoCollision")
  (Development|PrintText "Disabled River"))

(fn ConstructionScript)