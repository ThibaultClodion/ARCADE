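; BP_Boss1 is a boss actor with a health pool and an on-screen health widget created on BeginPlay.
; Hits on its Electric_meter component deal damage equal to the speed of the actor that struck it.
; Each hit spawns Niagara smoke at the SmokePoints actors.
; At or below LowHealth, sparks spawn once at the ElectricPoints actors, guarded by a flag; no death handling is present.
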(event OnComponentHit(Electric_meter)
  (params (HitComponent :type Primitive%20Component%20Object%20Reference) (OtherActor :type Actor%20Object%20Reference) (OtherComp :type Primitive%20Component%20Object%20Reference) (NormalImpulse :type Vector :default "0, 0, 0") (Hit :type Hit%20Result%20Structure%20%28by%20ref%29))
  (CallFunction|TakeDamage (Math|Vector|VectorLength (Transformation|GetVelocity OtherActor))))

(event EventBeginPlay
  (Variables|Default|SetHealth (Variables|Default|GetMaxHealth))
  (CallFunction|CreateLifeWidget))

(fn ConstructionScript)

(fn SpawnSmokes
  (for _array_element (Variables|Default|GetSmokePoints)
    (Niagara|SpawnSystematLocation "/Game/Effects/NS_Smoke.NS_Smoke" (Transformation|GetActorLocation _array_element))))

(fn TakeDamage
  (params (Damage :type Float%20%28double-precision%29))
  (bind _output_get (Variables|Default|SetHealth (- (Variables|Default|GetHealth) Damage)))
  (CallFunction|SpawnSmokes)
  (if (<= _output_get (Variables|Default|GetLowHealth))
    (CallFunction|SpawnSparks)))

(fn CreateLifeWidget
  (bind _returnvalue (UserInterface|CreateWidget "/Game/Blueprints/Boss_1/WBP_Health_Boss1.WBP_Health_Boss1_C"))
  (UserInterface|Viewport|AddtoViewport _returnvalue 0)
  (Variables|Default|SetWidget_Health _returnvalue))

(fn SpawnSparks
  (if (not (Variables|Default|GetAlreadySpawnSparks))
    (for _array_element (Variables|Default|GetElectricPoints)
      (Niagara|SpawnSystematLocation "/Game/Effects/NS_Sparks.NS_Sparks" (Transformation|GetActorLocation _array_element))
      (Variables|Default|SetAlreadySpawnSparks true))))