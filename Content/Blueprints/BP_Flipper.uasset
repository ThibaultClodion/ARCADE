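; BP_Flipper is a pinball-style flipper that swings between two yaw angles when Flip and Flop events are triggered.
; The events only toggle an IsFlip flag, and Tick passes the raised or resting angle to RotateFlipperTo.
; That function eases CubePivot's relative rotation toward the target with a delta-time lerp scaled by FlipSpeedFactor, using a swept move.
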(event Custom|Flop
  (Variables|Default|SetIsFlip false))

(event Custom|Flip
  (Variables|Default|SetIsFlip true))

(event EventTick
  (params (DeltaSeconds :type Float%20%28single-precision%29))
  (if (Variables|Default|GetIsFlip)
    (CallFunction|RotateFlipperto "0.000000,-27.000000,0.000000")
    (else
      (CallFunction|RotateFlipperto "0.000000,20.000000,0.000000"))))

(fn ConstructionScript)

(fn RotateFlipperto
  (params (Rotation :type Rotator))
  (Transformation|SetRelativeRotation (Variables|Default|GetCubePivot) (Math|Rotator|Lerp(Rotator) (Variables|/Script/Engine.SceneComponent|GetRelativeRotation (Variables|Default|GetCubePivot)) Rotation (* (Utilities|Time|GetWorldDeltaSeconds) (Variables|Default|GetFlipSpeedFactor))) true false))