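; BP_CleanPetrol is a Boss3 trigger that cleans petrol off the ball and hurts the boss when it does.
; When a BP_Ball flagged as on petrol enters its box, GetPetrolOff clears that flag and restores the ball's default material.
; It then finds the BP_Boss with GetActorOfClass and calls its TakeDamage with the Damage value.
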(event OnComponentBeginOverlap(Box)
  (params (OverlappedComponent :type Primitive%20Component%20Object%20Reference) (OtherActor :type Actor%20Object%20Reference) (OtherComp :type Primitive%20Component%20Object%20Reference) (OtherBodyIndex :type Integer) (bFromSweep :type Boolean) (SweepResult :type Hit%20Result%20Structure%20%28by%20ref%29))
  (bind _asbp_ball (Utilities|Casting|CastToBP_Ball OtherActor))
  (if (Variables|/Game/Blueprints/BP_Ball.BP_Ball_C|GetIsOnPetrol _asbp_ball)
    (CallFunction|GetPetrolOff _asbp_ball)
    (bind _returnvalue (Actor|GetActorOfClass "/Game/Blueprints/Boss/BP_Boss.BP_Boss_C"))
    (Default|TakeDamage _returnvalue (Variables|Default|GetDamage))))

(fn ConstructionScript)

(fn GetPetrolOff
  (params (Ball :type BP%20Ball%20Object%20Reference))
  (Variables|/Game/Blueprints/BP_Ball.BP_Ball_C|SetIsOnPetrol Ball false)
  (Rendering|Material|SetMaterial (Variables|/Game/Blueprints/BP_Ball.BP_Ball_C|GetSphere Ball) 0 "/Game/Materials/M_Ball.M_Ball"))