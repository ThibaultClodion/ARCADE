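; BP_Falling is a trigger in Map2 that relocates the ball to a lower, offset position while keeping its motion.
; When a BP_Ball overlaps the Box, it records the ball's velocity and location, then destroys it.
; It spawns a replacement BP_Ball at a fixed offset from that location and applies the saved velocity to the new ball's physics Sphere.
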(event OnComponentBeginOverlap(Box)
  (params (OverlappedComponent :type Primitive%20Component%20Object%20Reference) (OtherActor :type Actor%20Object%20Reference) (OtherComp :type Primitive%20Component%20Object%20Reference) (OtherBodyIndex :type Integer) (bFromSweep :type Boolean) (SweepResult :type Hit%20Result%20Structure%20%28by%20ref%29))
  (bind _asbp_ball (Utilities|Casting|CastToBP_Ball OtherActor))
  (Variables|Default|SetVitesse (Transformation|GetVelocity _asbp_ball))
  (Variables|Default|SetLocation (Transformation|GetActorLocation _asbp_ball))
  (Actor|DestroyActor OtherActor)
  (bind _returnvalue (Game|SpawnActorfromClass "/Game/Blueprints/BP_Ball.BP_Ball_C" (Math|Conversions|ToTransform(Vector) (+ (Variables|Default|GetLocation) "-400.000000,0.000000,-540.000000")) "Undefined" "MultiplyWithRoot" 0 0))
  (Physics|SetPhysicsLinearVelocity (Variables|/Game/Blueprints/BP_Ball.BP_Ball_C|GetSphere _returnvalue) (Variables|Default|GetVitesse) false "None"))

(fn ConstructionScript)