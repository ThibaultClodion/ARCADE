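; BP_Elevator is a trigger in Map2 that moves an overlapping actor, presumably the ball, to a placed TeleportLocation actor.
; One second after Box overlap, it disables physics on the referenced Ball and sweeps the overlapping actor to the target.
; After a brief delay, it restores Ball physics and applies an unscaled backward force.
; The overlapping actor is not class-checked, as the BP_Ball comparison is left unused.
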(event OnComponentBeginOverlap(Box)
  (params (OverlappedComponent :type Primitive%20Component%20Object%20Reference) (OtherActor :type Actor%20Object%20Reference) (OtherComp :type Primitive%20Component%20Object%20Reference) (OtherBodyIndex :type Integer) (bFromSweep :type Boolean) (SweepResult :type Hit%20Result%20Structure%20%28by%20ref%29))
  (bind _ball (Variables|Default|GetBall))
  (Utilities|FlowControl|Delay 1.0)
  (Physics|SetSimulatePhysics (Variables|/Game/Blueprints/BP_Ball.BP_Ball_C|GetSphere (Variables|Default|GetBall)) false)
  (Transformation|SetActorLocation OtherActor (Transformation|GetActorLocation (Variables|Default|GetTeleportLocation)) true false)
  (Utilities|FlowControl|Delay 0.2)
  (Physics|SetSimulatePhysics (Variables|/Game/Blueprints/BP_Ball.BP_Ball_C|GetSphere _ball) true)
  (Physics|AddForce (Variables|/Game/Blueprints/BP_Ball.BP_Ball_C|GetSphere _ball) (Class|KismetMathLibrary|VectorBackward) "None" false))

(event EventBeginPlay)

(event Collision|EventActorBeginOverlap
  (params (OtherActor :type Actor%20Object%20Reference)))

(event EventTick
  (params (DeltaSeconds :type Float%20%28single-precision%29)))

(fn ConstructionScript)