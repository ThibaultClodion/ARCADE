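; BP_Trash is a trash actor that loses one hit point (PV) each time something begins overlapping its Box, printing the value before and after.
; At zero it destroys itself; if flagged as Water, it also spawns the NS_Water Niagara effect and raises the referenced Pool actor 100 units.
; The lift is instant, as the lerp alpha is fixed at 1 and the Chronologie timeline never runs.
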(event OnComponentBeginOverlap(Box)
  (params (OverlappedComponent :type Primitive%20Component%20Object%20Reference) (OtherActor :type Actor%20Object%20Reference) (OtherComp :type Primitive%20Component%20Object%20Reference) (OtherBodyIndex :type Integer) (bFromSweep :type Boolean) (SweepResult :type Hit%20Result%20Structure%20%28by%20ref%29))
  (bind _pool (Variables|Default|GetPool))
  (bind _returnvalue (Transformation|GetActorLocation _pool))
  (Development|PrintString (Utilities|String|ToString(Integer) (Variables|Default|GetPV)))
  (bind _result (Math|Integer|DecrementInt (Math|Conversions|ToInteger(Byte) (Variables|Default|GetPV)))
    (:%20%20
      (Variables|Default|SetPV (Class|KismetMathLibrary|ToInt64(Integer) _result))
      (Development|PrintString (Utilities|String|ToString(Integer) (Variables|Default|GetPV)))
      (if (== (Variables|Default|GetPV) 0)
        (Actor|DestroyActor)
        (if (Variables|Default|GetWater)
          (Niagara|SpawnSystematLocation "/Game/Effects/NS_Water.NS_Water" (Transformation|GetActorLocation))
          (if (Utilities|IsValid (Variables|Default|GetPool))
            (Transformation|SetActorLocation _pool (Math|Vector|Lerp(Vector) _returnvalue (+ _returnvalue (Math|Vector|MakeVector 0.0 0.0 1e+02)) 1.0) false false)))))))

(fn ConstructionScript)