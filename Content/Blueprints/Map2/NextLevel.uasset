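; NextLevel is a level-progression Blueprint that tracks trash cleanup and moves the game on to a boss level.
; Each Cleaning event increments the trash count and updates the remaining count from the total.
; When the count equals the total, it opens Boss2 if the Map2 flag is set, otherwise Boss4.
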(event Custom|Cleaning
  (bind _result (Math|Integer|IncrementInt (Variables|Default|GetNbTrash))
    (:%20%20
      (Variables|Default|SetRestants (- (Variables|Default|GetTotal) (Variables|Default|GetNbTrash)))
      (if (== _result (Variables|Default|GetTotal))
        (if (Variables|Default|GetMap2)
          (Game|OpenLevel(byObjectReference) "/Game/Maps/Boss2.Boss2")
          (else
            (Game|OpenLevel(byObjectReference) "/Game/Maps/Boss4.Boss4")))))))

(event EventBeginPlay)

(event Collision|EventActorBeginOverlap
  (params (OtherActor :type Actor%20Object%20Reference)))

(fn ConstructionScript)