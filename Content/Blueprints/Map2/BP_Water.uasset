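; Water actor for Map2 that rises in steps as trash actors are destroyed.
; Verification polls five trash references with IsActorBeingDestroyed; a hit calls TrashDestroyed, which lifts the water and increments the Dechets counter.
; It re-calls itself without delay until the counter reaches two, then prints a success message.
; Nothing here starts Verification, as BeginPlay is empty.
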(event Custom|TrashDestroyed
  (Transformation|SetActorLocation (+ (Transformation|GetActorLocation) (Math|Vector|MakeVector 0.0 0.0 2e+01)) false false)
  (bind _result (Math|Integer|IncrementInt (Variables|Default|GetDechets))
    (:%20%20
      (Variables|Default|SetDechets _result))))

(event Custom|Verification
  (if (== (Variables|Default|GetDechets) 2)
    (Development|PrintString "C'est good")
    (elif (Game|IsActorBeingDestroyed (Variables|Default|GetTrash))
      (CallFunction|TrashDestroyed)
      (CallFunction|Verification)
      (elif (Game|IsActorBeingDestroyed (Variables|Default|GetTrash2))
        (CallFunction|TrashDestroyed)
        (CallFunction|Verification)
        (elif (Game|IsActorBeingDestroyed (Variables|Default|GetTrash3))
          (CallFunction|TrashDestroyed)
          (CallFunction|Verification)
          (elif (Game|IsActorBeingDestroyed (Variables|Default|GetTrash4))
            (CallFunction|TrashDestroyed)
            (CallFunction|Verification)
            (elif (Game|IsActorBeingDestroyed (Variables|Default|GetTrash5))
              (CallFunction|TrashDestroyed)
              (CallFunction|Verification)
              (else
                (CallFunction|Verification)))))))))

(event EventBeginPlay)

(event Collision|EventActorBeginOverlap
  (params (OtherActor :type Actor%20Object%20Reference)))

(event EventTick
  (params (DeltaSeconds :type Float%20%28single-precision%29)))

(fn ConstructionScript)