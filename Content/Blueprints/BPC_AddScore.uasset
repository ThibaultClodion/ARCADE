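; BPC_AddScore is an actor component that awards points in the flipper (pinball) game whenever its owner's root primitive is hit.
; Each hit adds the current Scores entry to GI_Flipper and refreshes the game mode's score widget.
; An animated WBP_AddScore popup appears at the owner's screen-projected position, captured at BeginPlay.
; The score index then advances through the array, wrapping or holding at the last entry depending on AreScoresOnRepeat.
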(event Custom|OnRootHit
  (params (HitComponent :type Primitive%20Component%20Object%20Reference) (OtherActor :type Actor%20Object%20Reference) (OtherComp :type Primitive%20Component%20Object%20Reference) (NormalImpulse :type Vector) (Hit :type Hit%20Result%20Structure%20%28by%20ref%29))
  ;[1 0.4192 0.2891] Add score on hit and update score
  (CallFunction|Hit))

(event EventBeginPlay
  ;[0.5204 1 0.7252] Get the owner onHit event
  (bind _asprimitive_component (Utilities|Casting|CastToPrimitiveComponent (Variables|/Script/Engine.Actor|GetRootComponent (Components|GetOwner))))
  (Collision|BindEventtoOnComponentHit _asprimitive_component (delegate Custom|OnRootHit))
  (Variables|Default|SetWorldPosition (Transformation|GetWorldLocation _asprimitive_component)))

(fn GetScoretoAdd
  (return (Utilities|Array|Get(acopy) (Variables|Default|GetScores) (Variables|Default|GetScoreAugmentationIndex))))

(fn GetNextScore
  ;[1 1 1] Get the next score by changing the index
  (bind _result (Math|Integer|IncrementInt (Variables|Default|GetScoreAugmentationIndex))
    (:%20%20
      (Variables|Default|SetScoreAugmentationIndex _result)
      (if (not (Utilities|Array|IsValidIndex (Variables|Default|GetScores) (Variables|Default|GetScoreAugmentationIndex)))
        (if (Variables|Default|GetAreScoresOnRepeat)
          (Variables|Default|SetScoreAugmentationIndex 0)
          (else
            (bind _result_2 (Math|Integer|DecrementInt (Variables|Default|GetScoreAugmentationIndex))
              (:%20%20
                (Variables|Default|SetScoreAugmentationIndex _result_2)))))))))

(fn DisplayScore
  (params (ScoreToDisplay :type Integer))
  (bind _returnvalue (Game|GetPlayerController 0))
  (bind _returnvalue_2 (UserInterface|CreateWidget "/Game/UI/WBP_AddScore.WBP_AddScore_C" _returnvalue))
  (bind _output_get (LocalVariables|SetWidget _returnvalue_2))
  (Default|SetScore _output_get ScoreToDisplay)
  (UserInterface|Viewport|AddtoViewport _output_get 0)
  (Class|UserWidget|SetPositioninViewport _output_get (.ScreenPosition (Class|GameplayStatics|ProjectWorldtoScreen _returnvalue (Variables|Default|GetWorldPosition) false)) true)
  (UserInterface|Animation|PlayAnimation _output_get (Variables|/Game/UI/WBP_AddScore.WBP_AddScore_C|GetScoreAnim (LocalVariables|GetWidget)) 0.0 1 "Forward" 1.0 false))

(fn Hit
  (bind _score (CallFunction|GetScoretoAdd))
  (bind _asgi_flipper (Utilities|Casting|CastToGI_Flipper (Game|GetGameInstance)))
  (Default|AddScore _asgi_flipper _score)
  (CallFunction|DisplayScore _score)
  (CallFunction|UpdateWidgetScore)
  (CallFunction|GetNextScore))

(fn UpdateWidgetScore
  (bind _asgame_mode_flipper (Utilities|Casting|CastToGameMode_Flipper (Game|GetGameMode)))
  (Default|UpdateScore (Variables|/Game/Blueprints/Game/GameMode_Flipper.GameMode_Flipper_C|GetScoreWidget _asgame_mode_flipper)))