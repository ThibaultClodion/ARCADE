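; BP_ElectricSphere is a Boss 4 sphere that electrifies a BP_Ball it hits, then destroys itself.
; On any mesh hit, a BP_Ball gets the electric material and its IsElectric flag set.
; The hit also plays an electric sound at world origin and calls HideElectricity(false) on the BP_Boss cached at BeginPlay.
; A custom DestroyActor function spawns the electricity Niagara effect at the sphere before removing it.
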(event OnComponentHit(StaticMesh)
  (params (HitComponent :type Primitive%20Component%20Object%20Reference) (OtherActor :type Actor%20Object%20Reference) (OtherComp :type Primitive%20Component%20Object%20Reference) (NormalImpulse :type Vector :default "0, 0, 0") (Hit :type Hit%20Result%20Structure%20%28by%20ref%29))
  (CallFunction|SetBallonElectricState OtherActor)
  (Audio|SpawnSoundatLocation "/Game/Sounds/Boss/MS_Electric.MS_Electric" "0, 0, 0" "0, 0, 0" 1.0 1.0 0.0 0 0)
  (Default|HideElectricity (Variables|Default|GetBoss) false)
  (CallFunction|DestroyActor))

(event EventBeginPlay
  (CallFunction|GetBoss))

(fn ConstructionScript)

(fn DestroyActor
  (Niagara|SpawnSystematLocation "/Game/Effects/NS_Electricity.NS_Electricity" (Transformation|GetActorLocation))
  (Actor|DestroyActor))

(fn SetBallonElectricState
  (params (Ball :type Object%20Object%20Reference))
  (bind _asbp_ball (Utilities|Casting|CastToBP_Ball Ball))
  (Rendering|Material|SetMaterial (Variables|/Game/Blueprints/BP_Ball.BP_Ball_C|GetSphere _asbp_ball) 0 (Variables|Default|GetElectricMaterial))
  (Variables|/Game/Blueprints/BP_Ball.BP_Ball_C|SetIsElectric _asbp_ball true))

(fn GetBoss
  (bind _returnvalue (Actor|GetActorOfClass "/Game/Blueprints/Boss/BP_Boss.BP_Boss_C"))
  (Variables|Default|SetBoss _returnvalue))