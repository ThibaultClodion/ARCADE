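; BP_TrapBarrel is a destructible barrel for the Boss 2 fight that damages the boss when hit.
; Its Hit event applies damage to the BP_Boss found in the level, spawns a Niagara petrol leak, notifies BPCAddScore and destroys the barrel.
; On a random coin flip, it also spawns a BP_Ball at a set height and pushes it with a force in a random direction.
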(event Collision|EventHit
  (params (MyComp :type Primitive%20Component%20Object%20Reference) (Other :type Actor%20Object%20Reference) (OtherComp :type Primitive%20Component%20Object%20Reference) (bSelfMoved :type Boolean) (HitLocation :type Vector :default "0, 0, 0") (HitNormal :type Vector :default "0, 0, 0") (NormalImpulse :type Vector :default "0, 0, 0") (Hit :type Hit%20Result%20Structure%20%28by%20ref%29))
  (bind _returnvalue (Actor|GetActorOfClass "/Game/Blueprints/Boss/BP_Boss.BP_Boss_C"))
  (Default|TakeDamage _returnvalue (Variables|Default|GetDamage))
  (CallFunction|SpawnPetrolParticles)
  (Default|Hit (Variables|Default|GetBPC_AddScore))
  (if (Math|Random|RandomBool)
    (CallFunction|SpawnABall))
  (Actor|DestroyActor))

(fn ConstructionScript)

(fn SpawnPetrolParticles
  (Niagara|SpawnSystematLocation "/Game/Effects/NS_PetrolLeak.NS_PetrolLeak" (Transformation|GetActorLocation)))

(fn SpawnABall
  (bind _returnvalue (Transformation|GetActorLocation))
  (bind _returnvalue_2 (Game|SpawnActorfromClass "/Game/Blueprints/BP_Ball.BP_Ball_C" (Math|Transform|MakeTransform (Math|Vector|MakeVector (.x _returnvalue) (.y _returnvalue) (Variables|Default|GetZSpawnOffset)) "0, 0, 0" "1.000000,1.000000,1.000000") "Undefined" "MultiplyWithRoot" 0 0))
  (Physics|AddForce (Variables|/Game/Blueprints/BP_Ball.BP_Ball_C|GetSphere _returnvalue_2) (* (Math|Random|RandomUnitVector) (Variables|Default|GetSpawnForceScale)) "None" false))