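; BP_Boss is a boss with a health widget that takes damage when hit on its Electric_meter and opens the next level once health drops below zero.
; Damage equals the hitting ball's speed, gated by hittable and electric-only flags.
; An electric-only hit drains the ball's charge and spawns a new electricity sphere at a random point.
; Hits blink the red eye and emit particles, with one-time sparks at low health.
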(event OnComponentHit(Electric_meter)
  (params (HitComponent :type Primitive%20Component%20Object%20Reference) (OtherActor :type Actor%20Object%20Reference) (OtherComp :type Primitive%20Component%20Object%20Reference) (NormalImpulse :type Vector :default "0, 0, 0") (Hit :type Hit%20Result%20Structure%20%28by%20ref%29))
  (bind _isdamageable (CallFunction|CanbeDamaged OtherActor))
  (if _isdamageable
    (CallFunction|TakeDamage (CallFunction|GetDamage OtherActor))
    (Audio|SpawnSoundatLocation "/Game/Sounds/Boss/MS_Metal_Hit.MS_Metal_Hit" "0, 0, 0" "0, 0, 0" 1.0 1.0 0.0 0 0)))

(event Custom|EyeBlink
  (bind _counter (Utilities|FlowControl|DoN (Variables|Health|GetNbBlink) :!label _label)
    (:Exit
      (Development|SetHiddeninGame (Variables|Default|GetRedEye) (== (Math|Integer|%(Integer) _counter 2) 0) false)
      (Utilities|FlowControl|Delay 0.3)
      (if (== _counter (Variables|Health|GetNbBlink))
        (goto _label Reset)
        (else
          (goto _label))))))

(event EventBeginPlay
  (Variables|Health|SetHealth (Variables|Health|GetMaxHealth))
  (CallFunction|CreateLifeWidget)
  (CallFunction|HideEyeifNonHittable))

(fn ConstructionScript)

(fn SpawnSmokes
  (if (Variables|Health|GetIsHitOnlyByElectric)
    (Audio|PlaySoundatLocation "/Game/Sounds/Boss/MS_BigElectric.MS_BigElectric" "0, 0, 0" "0, 0, 0" 1.0 1.0 0.0 0 0 0 0)
    (else
      (Audio|PlaySoundatLocation "/Game/Sounds/Boss/MS_Steam.MS_Steam" "0, 0, 0" "0, 0, 0" 1.0 1.0 0.0 0 0 0 0)))
  (for _array_element (Variables|Particles|GetHitPoints)
    (Niagara|SpawnSystematLocation (Variables|Particles|GetHitParticle) (Transformation|GetActorLocation _array_element))))

(fn TakeDamage
  (params (Damage :type Float%20%28double-precision%29))
  (CallFunction|EyeBlink)
  (bind _output_get (Variables|Health|SetHealth (- (Variables|Health|GetHealth) Damage)))
  (CallFunction|SpawnSmokes)
  (if (<= _output_get (Variables|Health|GetLowHealth))
    (CallFunction|SpawnSparks)
    (if (< (Variables|Health|GetHealth) 0.0)
      (Game|OpenLevel(byObjectReference) (Variables|Default|GetNextLevel)))))

(fn CreateLifeWidget
  (bind _returnvalue (UserInterface|CreateWidget "/Game/Blueprints/Boss/WBP_Health_Boss.WBP_Health_Boss_C"))
  (UserInterface|Viewport|AddtoViewport _returnvalue 0)
  (Variables|Health|SetWidget_Health _returnvalue))

(fn SpawnSparks
  (if (not (Variables|Particles|GetAlreadySpawnSparks))
    (for _array_element (Variables|Particles|GetSparksPoints)
      (Niagara|SpawnSystematLocation "/Game/Effects/NS_Sparks.NS_Sparks" (Transformation|GetActorLocation _array_element))
      (Variables|Particles|SetAlreadySpawnSparks true))))

(fn GetDamage
  (params (Ball :type Actor%20Object%20Reference))
  (return (Math|Vector|VectorLength (Transformation|GetVelocity Ball))))

(fn CanbeDamaged
  (params (Ball :type Actor%20Object%20Reference))
  (if (Variables|Health|GetIsHittable)
    (if (Variables|Health|GetIsHitOnlyByElectric)
      ;[0.1779 1 0.6939] Test if ball is electric and disable electricity if it's the case
      (bind _asbp_ball (Utilities|Casting|CastToBP_Ball Ball))
      (if (Variables|/Game/Blueprints/BP_Ball.BP_Ball_C|GetIsElectric _asbp_ball)
        (CallFunction|DisableElectricityonBall _asbp_ball)
        (return true)
        (else
          (return false)))
      (else
        (return true)))
    (else
      (return false))))

(fn DisableElectricityonBall
  (params (Ball :type BP%20Ball%20Object%20Reference))
  (Rendering|Material|SetMaterial (Variables|/Game/Blueprints/BP_Ball.BP_Ball_C|GetSphere Ball) 0 "/Game/Materials/M_Ball.M_Ball")
  (CallFunction|SpawnNewElectricitySphere)
  (Variables|/Game/Blueprints/BP_Ball.BP_Ball_C|SetIsElectric Ball false)
  (CallFunction|HideElectricity true))

(fn SpawnNewElectricitySphere
  (Game|SpawnActorfromClass "/Game/Blueprints/Boss/Boss4/BP_ElectricSphere.BP_ElectricSphere_C" (Math|Transform|MakeTransform (Transformation|GetActorLocation (.OutItem (Utilities|Array|Random (Variables|Fight|GetElectricitySphereSpawns)))) "0, 0, 0" "1.000000,1.000000,1.000000") "Undefined" "MultiplyWithRoot" 0 0))

(fn HideEyeifNonHittable
  (if (Variables|Health|GetIsHitOnlyByElectric)
    (CallFunction|HideElectricity true)
    (Variables|Health|SetNbBlink 6)
    (elif (Variables|Health|GetIsHittable)
      (Variables|Health|SetNbBlink 7)
      (else
        (Variables|Health|SetNbBlink 8)
        (Development|SetHiddeninGame (Variables|Default|GetRedEye) true false)))))

(fn HideElectricity
  (params (Hide :type Boolean))
  (Development|SetHiddeninGame (Variables|Default|GetRedEye) Hide false)
  (bind _redlight (Variables|Default|GetRedLight)
    (:then
      (Rendering|SetActorHiddenInGame _redlight Hide))
    (:else)))