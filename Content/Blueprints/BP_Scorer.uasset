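; BP_Scorer is a scoring target, apparently for a pinball-style flipper game, that awards points when an actor overlaps it.
; On overlap it reads the points from its BPCAddScore component, adds them through GameMode_Flipper and plays an arcade sound.
; It then blinks its Scorer mesh three times by swapping materials between chained delays, with no filter on the overlapping actor.
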(event Collision|EventActorBeginOverlap
  (params (OtherActor :type Actor%20Object%20Reference))
  (bind _duration (Variables|Default|GetDuration))
  (bind _asgame_mode_flipper (Utilities|Casting|CastToGameMode_Flipper (Game|GetGameMode)))
  (bind _score (Default|GetScoretoAdd (Variables|Default|GetBPC_AddScore)))
  (Default|AddScore _asgame_mode_flipper _score)
  (Audio|PlaySound2D "/Game/Effects/arcade-ui-7-229506.arcade-ui-7-229506" 0.25 1.0 0.0 0 0)
  (Rendering|Material|SetMaterial (Variables|Default|GetScorer) 0 "/Engine/EngineDebugMaterials/DebugMeshMaterialFakeLight.DebugMeshMaterialFakeLight")
  (Utilities|FlowControl|Delay _duration)
  (Rendering|Material|SetMaterial (Variables|Default|GetScorer) 0 "/Engine/TemplateResources/MI_Template_BaseGray_02_Metal.MI_Template_BaseGray_02_Metal")
  (Utilities|FlowControl|Delay _duration)
  (Rendering|Material|SetMaterial (Variables|Default|GetScorer) 0 "/Engine/EngineDebugMaterials/DebugMeshMaterialFakeLight.DebugMeshMaterialFakeLight")
  (Utilities|FlowControl|Delay _duration)
  (Rendering|Material|SetMaterial (Variables|Default|GetScorer) 0 "/Engine/TemplateResources/MI_Template_BaseGray_02_Metal.MI_Template_BaseGray_02_Metal")
  (Utilities|FlowControl|Delay _duration)
  (Rendering|Material|SetMaterial (Variables|Default|GetScorer) 0 "/Engine/EngineDebugMaterials/DebugMeshMaterialFakeLight.DebugMeshMaterialFakeLight")
  (Utilities|FlowControl|Delay _duration)
  (Rendering|Material|SetMaterial (Variables|Default|GetScorer) 0 "/Engine/TemplateResources/MI_Template_BaseGray_02_Metal.MI_Template_BaseGray_02_Metal"))

(fn ConstructionScript)