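; BP_Map3Purifier is an overlap-triggered purifier on Map 3 that counts progress toward the boss zone.
; First activation swaps the pad material, stops Niagara, increments the game instance count, then updates the widget and score if the widget is ready.
; Every second purifier reveals a tagged hidden wind turbine.
; The eighth async-loads Boss1, then opens Boss3.
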(event EventBeginPlay
  (bind _asgi_flipper (Utilities|Casting|CastToGI_Flipper (Game|GetGameInstance)))
  (bind _outactors (Actor|GetAllActorswithTag "HiddenWindTurbine"))
  (Variables|Default|SetObjectList _outactors))

(event Collision|EventActorBeginOverlap
  (params (OtherActor :type Actor%20Object%20Reference))
  (Rendering|Material|SetMaterial (Variables|Default|GetPad%20) 0 "/Game/Materials/M_Purified.M_Purified")
  (if (not (Variables|Default|GetActivated))
    (Variables|Default|SetActivated true)
    (Math|Integer|IncrementInt (Variables|/Game/Blueprints/Game/GI_Flipper.GI_Flipper_C|GetPurifiersMap3 (stale EventBeginPlay _asgi_flipper))
      (:%20%20
        (Components|Activation|Deactivate (Variables|Default|GetNiagara))
        (bind _outactors (Actor|GetAllActorsOfClass "BP_Map3Purifier_C"))
        (Variables|/Game/Blueprints/Game/GI_Flipper.GI_Flipper_C|SetPurifiersMap3Count (stale EventBeginPlay _asgi_flipper) (Utilities|Array|Length _outactors))
        (bind _asgame_mode_flipper (Utilities|Casting|CastToGameMode_Flipper (Game|GetGameMode)))
        (if (Variables|/Game/Blueprints/Game/GameMode_Flipper.GameMode_Flipper_C|GetWidgetReady _asgame_mode_flipper)
          (Default|UpdatePurifiers (Variables|/Game/Blueprints/Game/GameMode_Flipper.GameMode_Flipper_C|GetPurifiersWidget _asgame_mode_flipper))
          (Audio|PlaySound2D "/Engine/VREditor/Sounds/UI/Enter_Play.Enter_Play" 0.2 0.6 0.0 0 0 false)
          (Utilities|Casting|CastToGI_Flipper (Game|GetGameInstance))
          (Default|Hit (Variables|Default|GetBPC_AddScore))
          (Math|Integer|CompareInt (Variables|/Game/Blueprints/Game/GI_Flipper.GI_Flipper_C|GetPurifiersMap3 (stale EventBeginPlay _asgi_flipper)) 8
            (:==
              (Development|PrintText "Entering boss zone...")
              (Utilities|AsyncLoadAsset "/Game/Maps/Boss1.Boss1"
                (:Completed
                  (Game|OpenLevel(byObjectReference) "/Game/Maps/Boss3.Boss3"))))
            (:<
              (Math|Integer|CompareInt (Math|Integer|%(Integer) (Variables|/Game/Blueprints/Game/GI_Flipper.GI_Flipper_C|GetPurifiersMap3 (stale EventBeginPlay _asgi_flipper)) 2)
                (:==
                  (Rendering|SetActorHiddenInGame (Utilities|Array|Get(acopy) (Variables|Default|GetObjectList) (/ (Variables|/Game/Blueprints/Game/GI_Flipper.GI_Flipper_C|GetPurifiersMap3 (stale EventBeginPlay _asgi_flipper)) 2)) false)
                  (Audio|PlaySound2D "/Game/Effects/mixkit-garage-pneumatic-screwer-817.mixkit-garage-pneumatic-screwer-817" 0.1 0.8 0.0 0 0))))))))))

(fn ConstructionScript)